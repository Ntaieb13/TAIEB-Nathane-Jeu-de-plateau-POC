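; GM_Memory is the Blueprint for a memory card game that handles pair matching when cards are clicked.
; OnCardClicked stores the first card in PrevCard, then compares the second card's Color to it as integers through TestPair.
; A match adds a point through UpdateScore and destroys both cards, while a mismatch calls TurnCard on both immediately.
; PrevCard clears after each comparison.
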(event EventBeginPlay)

(event EventTick
  (params (DeltaSeconds :type Float%20%28single-precision%29)))

(fn ConstructionScript)

(fn OnCardClicked
  (params (Card :type BP%20Card%20Object%20Reference))
  (if (Utilities|IsValid (Variables|Default|GetPrevCard))
    (bind _returnvalue (Class|MemoryGM|TestPair (Math|Conversions|ToInteger(Byte) (Variables|/Game/Memory/Blueprint/BP_Card.BP_Card_C|GetColor Card)) (Math|Conversions|ToInteger(Byte) (Variables|/Game/Memory/Blueprint/BP_Card.BP_Card_C|GetColor (Variables|Default|GetPrevCard)))))
    (if _returnvalue
      (Class|MemoryGM|UpdateScore 1)
      (Actor|DestroyActor Card)
      (Actor|DestroyActor (Variables|Default|GetPrevCard))
      (else
        (Class|MemoryCard|TurnCard Card)
        (Class|MemoryCard|TurnCard (Variables|Default|GetPrevCard))))
    (Variables|Default|SetPrevCard 0)
    (else
      (Variables|Default|SetPrevCard Card))))