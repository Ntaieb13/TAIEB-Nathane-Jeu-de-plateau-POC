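; Clickable card actor for a Memory game, with a colour-coded Verso face.
; The construction script sets the Verso material from the Color variable.
; A click on a clickable card calls TurnCard, waits briefly, then reports the card to GM_Memory, cached at BeginPlay.
; ToggleCard inverts clickability and flips the root's roll between face orientations.
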(event EventBeginPlay
  (bind _asgm_memory (Utilities|Casting|CastToGM_Memory (Game|GetGameMode)))
  (Variables|Default|SetAs%20GM%20Memory _asgm_memory))

(event Collision|EventActorBeginOverlap
  (params (OtherActor :type Actor%20Object%20Reference)))

(event EventTick
  (params (DeltaSeconds :type Float%20%28single-precision%29)))

(event MouseInput|EventActorOnClicked
  (params (ButtonPressed :type Key%20Structure :default "None"))
  (if (Variables|Default|GetbIsClickable)
    (Class|MemoryCard|TurnCard)
    (Utilities|FlowControl|Delay 0.5)
    (Default|OnCardClicked (Variables|Default|GetAs%20GM%20Memory) self)))

(fn ConstructionScript
  (CallFunction|ChangeCardColor))

(fn ChangeCardColor
  (switch Utilities|FlowControl|Switch|SwitchonE_CardColor (Variables|Default|GetColor)
    (:NewEnumerator0
      (Rendering|Material|SetMaterial (Variables|Default|GetVerso) 0 "/Game/Memory/Blueprint/MI_Yellow.MI_Yellow"))
    (:NewEnumerator1
      (Rendering|Material|SetMaterial (Variables|Default|GetVerso) 0 "/Game/Memory/Blueprint/MI_Red.MI_Red"))
    (:NewEnumerator2
      (Rendering|Material|SetMaterial (Variables|Default|GetVerso) 0 "/Game/Memory/Blueprint/MI_Blue.MI_Blue"))
    (:NewEnumerator3
      (Rendering|Material|SetMaterial (Variables|Default|GetVerso) 0 "/Game/Memory/Blueprint/MI_Green.MI_Green"))))

(fn ToggleCard
  (Variables|Default|SetisClickable (not (Variables|Default|GetisClickable)))
  (if (== (.roll (Transformation|GetWorldRotation (Variables|Default|GetDefaultSceneRoot))) 0.0)
    (Transformation|SetRelativeRotation (Variables|Default|GetDefaultSceneRoot) (Math|Rotator|MakeRotator 1.8e+02 0.0 0.0) false false)
    (else
      (Transformation|SetRelativeRotation (Variables|Default|GetDefaultSceneRoot) (Math|Rotator|MakeRotator 0.0 0.0 0.0) false false))))